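; BP_Player is the player pawn of a banana collecting game, moved by axis input and tinted as it collects.
; MoveForward and MoveRight add speed-scaled input along the actor's forward and right vectors, which Tick consumes as a swept, delta-time-scaled local offset.
; Overlapping a BP_Banana destroys it and increments a counter, which drives the clamped ColorAlpha parameter on a dynamic M_Cube material created at BeginPlay.
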(event EventBeginPlay
  (bind _returnvalue (Rendering|Material|CreateDynamicMaterialInstance (Variables|Default|GetStaticMesh) 0 "/Game/BananaCollector/Materials/M_Cube.M_Cube" "None" :!class /Script/Engine.PrimitiveComponent))
  (Variables|Default|SetCubeMaterial _returnvalue))

(event EventTick
  (params (DeltaSeconds :type Float%20%28single-precision%29))
  (bind _returnvalue (Class|Pawn|ConsumeMovementInputVector))
  (Transformation|AddActorLocalOffset (* _returnvalue DeltaSeconds) true false))

(event Collision|EventActorBeginOverlap
  (params (OtherActor :type Actor%20Object%20Reference))
  (bind _asbp_banana (Utilities|Casting|CastToBP_Banana OtherActor))
  (Actor|DestroyActor _asbp_banana)
  (bind _result (Math|Float|IncrementFloat (Variables|Default|GetBananaCounter))
    (:%20%20
      (Rendering|Material|SetScalarParameterValue (Variables|Default|GetCubeMaterial) "ColorAlpha" (Math|Float|Clamp(Float) (/ _result 9.0)) :!class /Script/Engine.MaterialInstanceDynamic))))

(event Input|AxisEvents|InputAxisMoveForward
  (params (AxisValue :type Float%20%28single-precision%29))
  (Pawn|Input|AddMovementInput (Transformation|GetActorForwardVector) (* AxisValue (Variables|Default|GetMaxSpeed)) false))

(event Input|AxisEvents|InputAxisMoveRight
  (params (AxisValue :type Float%20%28single-precision%29))
  (Pawn|Input|AddMovementInput (Transformation|GetActorRightVector) (* AxisValue (Variables|Default|GetMaxSpeed)) false))

(fn ConstructionScript)